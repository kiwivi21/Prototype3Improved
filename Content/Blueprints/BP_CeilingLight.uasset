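; BP_CeilingLight is a ceiling light actor that flickers while a BP_Spook is nearby.
; A detection box sets a SpookIsNear flag on overlap begin and clears it on overlap end.
; While the flag is set, Tick calls Flicker every frame, and the random Delay after it feeds nothing, so it doesn't throttle calls.
; Flicker uses timed delays to step the rect light's intensity and swap the mesh between grey and emissive materials.
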(event OnComponentBeginOverlap(DetectionBox)
  (params (OverlappedComponent :type Primitive%20Component%20Object%20Reference) (OtherActor :type Actor%20Object%20Reference) (OtherComp :type Primitive%20Component%20Object%20Reference) (OtherBodyIndex :type Integer) (bFromSweep :type Boolean) (SweepResult :type Hit%20Result%20Structure%20%28by%20ref%29))
  (Utilities|Casting|CastToBP_Spook OtherActor)
  (Variables|Default|SetSpookIsNear true))

(event OnComponentEndOverlap(DetectionBox)
  (params (OverlappedComponent :type Primitive%20Component%20Object%20Reference) (OtherActor :type Actor%20Object%20Reference) (OtherComp :type Primitive%20Component%20Object%20Reference) (OtherBodyIndex :type Integer))
  (Utilities|Casting|CastToBP_Spook OtherActor)
  (Variables|Default|SetSpookIsNear false))

(event Custom|Flicker
  (bind _rectlight (Variables|Default|GetRectLight))
  (Rendering|Components|Light|SetIntensity _rectlight 1e+03)
  (Rendering|Material|SetMaterial (Variables|Default|GetStaticMesh) 0 "/Engine/EditorMeshes/ColorCalibrator/M_GreyBall.M_GreyBall")
  (Utilities|FlowControl|Delay 0.5)
  (Rendering|Components|Light|SetIntensity _rectlight 1.2e+04)
  (Utilities|FlowControl|Delay 0.4)
  (Rendering|Components|Light|SetIntensity _rectlight 1e+03)
  (Rendering|Material|SetMaterial (Variables|Default|GetStaticMesh) 0 "/Game/Assets/Materials/BaseMats/EmmissiveLight_MAT.EmmissiveLight_MAT")
  (Utilities|FlowControl|Delay 0.5)
  (Rendering|Components|Light|SetIntensity _rectlight 5e+03))

(event EventBeginPlay)

(event Collision|EventActorBeginOverlap
  (params (OtherActor :type Actor%20Object%20Reference)))

(event EventTick
  (params (DeltaSeconds :type Float%20%28single-precision%29))
  (if (Variables|Default|GetSpookIsNear)
    (CallFunction|Flicker)
    (Utilities|FlowControl|Delay (Math|Random|RandomFloatinRange 5.0 3e+01))))

(fn ConstructionScript)