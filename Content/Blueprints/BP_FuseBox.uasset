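; BP_FuseBox is an interactable horror-game quest object that takes a Fuse from the player's inventory and opens the elevator doors.
; Overlap events flag the player in range, and Tick polls the player's Interacting flag, requiring quest 2 or later.
; Inserting the fuse swaps to the full mesh, updates inventory, saves, and advances to quest 3.
; BeginPlay restores the filled state from the game instance's CompletedItems.
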(event EventBeginPlay
  (bind _asbp_first_person_character (Utilities|Casting|CastToBP_FirstPersonCharacter (Game|GetPlayerCharacter 0)))
  (Variables|Default|SetPlayerRef _asbp_first_person_character)
  (bind _asbp_horror_instance (Utilities|Casting|CastToBP_HorrorInstance (Game|GetGameInstance)))
  (for _array_element (Variables|/Game/Blueprints/BP_HorrorInstance.BP_HorrorInstance_C|GetCompletedItems _asbp_horror_instance)
    (if (Utilities|Enum|Equal(Enum) _array_element "Fuse")
      (Variables|Default|SetIsFull true)
      (Components|StaticMesh|SetStaticMesh (Variables|Default|GetFuseBox) "/Game/Assets/Models/Interactables/CommsRoom/Fuse_Full.Fuse_Full"))))

(event EventTick
  (params (DeltaSeconds :type Float%20%28single-precision%29))
  (bind _playerref (Variables|Default|GetPlayerRef))
  (bind _pickedup (Variables|/Game/FirstPerson/Blueprints/BP_FirstPersonCharacter.BP_FirstPersonCharacter_C|GetPickedUp _playerref))
  (if (Variables|Default|GetInRange)
    (if (Variables|/Game/FirstPerson/Blueprints/BP_FirstPersonCharacter.BP_FirstPersonCharacter_C|GetInteracting (Variables|Default|GetPlayerRef))
      (if (not (Variables|Default|GetIsFull))
        (bind _asbp_horror_instance (Utilities|Casting|CastToBP_HorrorInstance (Game|GetGameInstance)))
        (if (>= (Variables|/Game/Blueprints/BP_HorrorInstance.BP_HorrorInstance_C|GetQuestNumber _asbp_horror_instance) 2)
          (for _array_element (Variables|/Game/Blueprints/BP_HorrorInstance.BP_HorrorInstance_C|GetNamesInInventory _asbp_horror_instance)
            (if (Utilities|Enum|Equal(Enum) _array_element "Fuse")
              (Variables|Default|SetIsFull true)
              (Components|StaticMesh|SetStaticMesh (Variables|Default|GetFuseBox) "/Game/Assets/Models/Interactables/CommsRoom/Fuse_Full.Fuse_Full")
              (for _array_element_2 _pickedup
                (if (Utilities|Enum|Equal(Enum) (Variables|/Game/Blueprints/Inventory/ItemsForInventory/BP_ParentPickup.BP_ParentPickup_C|GetUniqueNameForInventory _array_element_2) "Fuse")
                  (Utilities|Array|RemoveItem _pickedup _array_element_2)
                  (Utilities|Array|RemoveItem (Variables|/Game/Blueprints/BP_HorrorInstance.BP_HorrorInstance_C|GetNamesInInventory _asbp_horror_instance) _array_element)
                  (Utilities|Array|AddUnique (Variables|/Game/Blueprints/BP_HorrorInstance.BP_HorrorInstance_C|GetCompletedItems _asbp_horror_instance) "Fuse")
                  (Default|Save _playerref)))))
          (if (Variables|Default|GetIsFull)
            (Development|PrintString "Done, let's talk to the man again")
            (Variables|/Game/Blueprints/BP_HorrorInstance.BP_HorrorInstance_C|SetQuestNumber _asbp_horror_instance 3)
            (Variables|/Game/Blueprints/BP_HorrorInstance.BP_HorrorInstance_C|SetQuestString _asbp_horror_instance "Quest 3: Talk to the man and see if everything is working")
            (bind _returnvalue (Actor|GetActorOfClass "/Game/Blueprints/Elevator/BP_ElevatorDoors.BP_ElevatorDoors_C"))
            (Default|OpenDoors _returnvalue)
            (else
              (Development|PrintString "There seems to be a fuse missing")))
          (else
            (Development|PrintString "There seems to be a fuse missing")))))))

(event Collision|EventActorEndOverlap
  (params (OtherActor :type Actor%20Object%20Reference))
  (if (== (Utilities|GetClass OtherActor) "/Game/FirstPerson/Blueprints/BP_FirstPersonCharacter.BP_FirstPersonCharacter_C")
    (Variables|Default|SetInRange false)))

(event Collision|EventActorBeginOverlap
  (params (OtherActor :type Actor%20Object%20Reference))
  (if (== (Utilities|GetClass OtherActor) "/Game/FirstPerson/Blueprints/BP_FirstPersonCharacter.BP_FirstPersonCharacter_C")
    (Variables|Default|SetInRange true)))

(fn ConstructionScript)