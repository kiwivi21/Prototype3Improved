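; BP_HideWardrobe is an interactable wardrobe that the player can hide in and step out of.
; Interact calls Hide, which flips IsInside and teleports the first player character to the InPos or OutPos component location without sweeping.
; StaticMesh collision toggles are present but disconnected, so they never run.
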(event Custom|Hide
  (if (Variables|Default|GetIsInside)
    (Variables|Default|SetIsInside false)
    (Transformation|SetActorLocation (Game|GetPlayerCharacter 0) (Transformation|GetWorldLocation (Variables|Default|GetOutPos)) false true)
    (else
      (Variables|Default|SetIsInside true)
      (Transformation|SetActorLocation (Game|GetPlayerCharacter 0) (Transformation|GetWorldLocation (Variables|Default|GetInPos)) false true))))

(event EventBeginPlay)

(event Collision|EventActorBeginOverlap
  (params (OtherActor :type Actor%20Object%20Reference)))

(event EventTick
  (params (DeltaSeconds :type Float%20%28single-precision%29)))

(event EventInteract
  (CallFunction|Hide))

(fn ConstructionScript)