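; BP_FallingBowl is a physics prop bowl that gets pushed when the player comes near and smashes on tagged surfaces.
; Overlap of the Detect component by BP_FirstPersonCharacter applies a velocity-change impulse to the bowl along the Arrow component's forward direction.
; When the bowl hits an actor whose root component is tagged "Smash", it plays audio and destroys itself after a short delay.
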(event OnComponentBeginOverlap(Detect)
  (params (OverlappedComponent :type Primitive%20Component%20Object%20Reference) (OtherActor :type Actor%20Object%20Reference) (OtherComp :type Primitive%20Component%20Object%20Reference) (OtherBodyIndex :type Integer) (bFromSweep :type Boolean) (SweepResult :type Hit%20Result%20Structure%20%28by%20ref%29))
  (Utilities|Casting|CastToBP_FirstPersonCharacter OtherActor)
  (Physics|AddImpulse (Variables|Default|GetBowl) (* (Math|Vector|GetForwardVector (Variables|Default|GetArrow)) 2e+02) "None" true))

(event OnComponentHit(Bowl)
  (params (HitComponent :type Primitive%20Component%20Object%20Reference) (OtherActor :type Actor%20Object%20Reference) (OtherComp :type Primitive%20Component%20Object%20Reference) (NormalImpulse :type Vector :default "0, 0, 0") (Hit :type Hit%20Result%20Structure%20%28by%20ref%29))
  (if (Components|ComponentHasTag (Variables|/Script/Engine.Actor|GetRootComponent OtherActor) "Smash")
    (Audio|Components|Audio|Play (Variables|Default|GetAudio) 0.0)
    (Utilities|FlowControl|Delay 0.1)
    (Actor|DestroyActor)))

(event EventBeginPlay)

(event Collision|EventActorBeginOverlap
  (params (OtherActor :type Actor%20Object%20Reference)))

(event EventTick
  (params (DeltaSeconds :type Float%20%28single-precision%29)))

(fn ConstructionScript)