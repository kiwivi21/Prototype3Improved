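; Parent pickup Blueprint for items that the first-person character collects by interacting while in range.
; Begin and end overlap with BP_FirstPersonCharacter toggle InRange, and Tick polls the character's Interacting flag until pickup.
; On pickup it hides Model and ignores its collisions instead of destroying the actor, then adds itself uniquely to the character's PickedUp array.
; GetPickedUp is an empty stub.
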(event EventBeginPlay)

(event Collision|EventActorBeginOverlap
  (params (OtherActor :type Actor%20Object%20Reference))
  (if (== (Utilities|GetClass OtherActor) "/Game/FirstPerson/Blueprints/BP_FirstPersonCharacter.BP_FirstPersonCharacter_C")
    (Variables|Default|SetInRange true)))

(event EventTick
  (params (DeltaSeconds :type Float%20%28single-precision%29))
  (if (not (Variables|Default|GetPickedUp))
    (if (Variables|Default|GetInRange)
      (bind _asbp_first_person_character (Utilities|Casting|CastToBP_FirstPersonCharacter (Game|GetPlayerCharacter 0)))
      (if (Variables|/Game/FirstPerson/Blueprints/BP_FirstPersonCharacter.BP_FirstPersonCharacter_C|GetInteracting _asbp_first_person_character)
        (Variables|Default|SetPickedUp true)
        (Rendering|SetVisibility (Variables|Default|GetModel) false false)
        (Collision|SetCollisionResponsetoAllChannels (Variables|Default|GetModel) "ECR_Ignore")
        (Utilities|Array|AddUnique (Variables|/Game/FirstPerson/Blueprints/BP_FirstPersonCharacter.BP_FirstPersonCharacter_C|GetPickedUp _asbp_first_person_character) self)))))

(event Collision|EventActorEndOverlap
  (params (OtherActor :type Actor%20Object%20Reference))
  (if (== (Utilities|GetClass OtherActor) "/Game/FirstPerson/Blueprints/BP_FirstPersonCharacter.BP_FirstPersonCharacter_C")
    (Variables|Default|SetInRange false)))

(fn ConstructionScript)

(fn GetPickedUp)