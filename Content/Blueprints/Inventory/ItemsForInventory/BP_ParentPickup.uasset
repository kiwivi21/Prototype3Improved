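; Base pickup actor for inventory items that the first-person character can collect and drop.
; Tick calls Collect when the overlapping player is interacting, hiding the model, disabling its collision and registering it with the character and game instance.
; BeginPlay re-collects items whose unique name is saved in the game instance's inventory list.
; GetDropped moves the model to the character's InventorySpawner, restores it and removes that saved name.
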(event Custom|Collect
  (Variables|Default|SetPickedUp true)
  (Rendering|SetVisibility (Variables|Default|GetModel) false false)
  (Collision|SetCollisionResponsetoAllChannels (Variables|Default|GetModel) "ECR_Ignore")
  (Utilities|Array|AddUnique (Variables|/Game/FirstPerson/Blueprints/BP_FirstPersonCharacter.BP_FirstPersonCharacter_C|GetPickedUp (Variables|Default|GetCharacterRef)) self)
  (Utilities|Array|AddUnique (Variables|/Game/Blueprints/BP_HorrorInstance.BP_HorrorInstance_C|GetNamesInInventory (Variables|Default|GetInstanceRef)) (Variables|Default|GetUniqueNameForInventory)))

(event EventBeginPlay
  (bind _asbp_first_person_character (Utilities|Casting|CastToBP_FirstPersonCharacter (Game|GetPlayerCharacter 0)))
  (Variables|Default|SetCharacterRef _asbp_first_person_character)
  (bind _asbp_horror_instance (Utilities|Casting|CastToBP_HorrorInstance (Game|GetGameInstance)))
  (bind _output_get (Variables|Default|SetInstanceRef _asbp_horror_instance))
  (for _array_element (Variables|/Game/Blueprints/BP_HorrorInstance.BP_HorrorInstance_C|GetNamesInInventory _output_get)
    (if (Utilities|Enum|Equal(Enum) _array_element (Variables|Default|GetUniqueNameForInventory))
      (CallFunction|Collect))))

(event Collision|EventActorBeginOverlap
  (params (OtherActor :type Actor%20Object%20Reference))
  (if (== (Utilities|GetClass OtherActor) "/Game/FirstPerson/Blueprints/BP_FirstPersonCharacter.BP_FirstPersonCharacter_C")
    (Variables|Default|SetInRange true)))

(event EventTick
  (params (DeltaSeconds :type Float%20%28single-precision%29))
  (if (not (Variables|Default|GetPickedUp))
    (if (Variables|Default|GetInRange)
      (if (Variables|/Game/FirstPerson/Blueprints/BP_FirstPersonCharacter.BP_FirstPersonCharacter_C|GetInteracting (Variables|Default|GetCharacterRef))
        (CallFunction|Collect)))))

(event Collision|EventActorEndOverlap
  (params (OtherActor :type Actor%20Object%20Reference))
  (if (== (Utilities|GetClass OtherActor) "/Game/FirstPerson/Blueprints/BP_FirstPersonCharacter.BP_FirstPersonCharacter_C")
    (Variables|Default|SetInRange false)))

(fn ConstructionScript)

(fn GetDropped
  (Transformation|SetWorldLocation (Variables|Default|GetModel) (Transformation|GetWorldLocation (Variables|/Game/FirstPerson/Blueprints/BP_FirstPersonCharacter.BP_FirstPersonCharacter_C|GetInventorySpawner (Variables|Default|GetCharacterRef))) false true)
  (Variables|Default|SetPickedUp false)
  (Rendering|SetVisibility (Variables|Default|GetModel) true false)
  (Collision|SetCollisionResponsetoAllChannels (Variables|Default|GetModel) "ECR_Overlap")
  (Utilities|Array|RemoveItem (Variables|/Game/Blueprints/BP_HorrorInstance.BP_HorrorInstance_C|GetNamesInInventory (Variables|Default|GetInstanceRef)) (Variables|Default|GetUniqueNameForInventory))
  (return self))