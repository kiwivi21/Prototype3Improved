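; BP_FinalDoor is a bulkhead door that opens once the player's quest progress reaches the seventh quest or later.
; On BeginPlay it caches the BP_HorrorInstance game instance, then polls its QuestNumber every Tick.
; When the threshold is met, an IsOpen flag makes it fire once, swapping the Door mesh to the open bulkhead variant and instantly rotating the Pivot a quarter turn.
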(event EventBeginPlay
  (bind _asbp_horror_instance (Utilities|Casting|CastToBP_HorrorInstance (Game|GetGameInstance)))
  (Variables|Default|SetInstanceRef _asbp_horror_instance))

(event Collision|EventActorBeginOverlap
  (params (OtherActor :type Actor%20Object%20Reference)))

(event EventTick
  (params (DeltaSeconds :type Float%20%28single-precision%29))
  (if (>= (Variables|/Game/Blueprints/BP_HorrorInstance.BP_HorrorInstance_C|GetQuestNumber (Variables|Default|GetInstanceRef)) 7)
    (if (not (Variables|Default|GetIsOpen))
      (Variables|Default|SetIsOpen true)
      (Components|StaticMesh|SetStaticMesh (Variables|Default|GetDoor) "/Game/Assets/Models/LevelKits/geo_bulkheadDoorOpen_01.geo_bulkheadDoorOpen_01")
      (Transformation|AddWorldRotation (Variables|Default|GetPivot) "0.000000,-90.000000,0.000000" false false))))

(fn ConstructionScript)