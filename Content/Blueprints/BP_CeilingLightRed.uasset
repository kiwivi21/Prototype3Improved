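; BP_CeilingLightRed is a ceiling light that spins its RectLight every tick and flickers while a BP_Spook is nearby.
; DetectionBox overlaps set a SpookIsNear flag, which makes Tick call Flicker every frame.
; Flicker steps the light intensity through timed delays, with a small random chance to play pitch-varied audio and activate sparks.
; The random Delay after Flicker has nothing wired after it, so it does not throttle the flicker.
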(event OnComponentBeginOverlap(DetectionBox)
  (params (OverlappedComponent :type Primitive%20Component%20Object%20Reference) (OtherActor :type Actor%20Object%20Reference) (OtherComp :type Primitive%20Component%20Object%20Reference) (OtherBodyIndex :type Integer) (bFromSweep :type Boolean) (SweepResult :type Hit%20Result%20Structure%20%28by%20ref%29))
  (Utilities|Casting|CastToBP_Spook OtherActor)
  (Variables|Default|SetSpookIsNear true))

(event OnComponentEndOverlap(DetectionBox)
  (params (OverlappedComponent :type Primitive%20Component%20Object%20Reference) (OtherActor :type Actor%20Object%20Reference) (OtherComp :type Primitive%20Component%20Object%20Reference) (OtherBodyIndex :type Integer))
  (Utilities|Casting|CastToBP_Spook OtherActor)
  (Variables|Default|SetSpookIsNear false))

(event Custom|Flicker
  (bind _rectlight (Variables|Default|GetRectLight))
  (Rendering|Components|Light|SetIntensity _rectlight 1e+02)
  (if (> (Math|Random|RandomIntegerinRange 0 100) 98)
    (Audio|Components|Audio|SetPitchMultiplier (Variables|Default|GetAudio) (Math|Random|RandomFloatinRange 0.0 1.0))
    (Audio|Components|Audio|Play (Variables|Default|GetAudio) 0.0)
    (Components|Activation|Activate (Variables|Default|GetSparks) true))
  (Utilities|FlowControl|Delay 0.5)
  (Rendering|Components|Light|SetIntensity _rectlight 5e+03)
  (Utilities|FlowControl|Delay 0.4)
  (Rendering|Components|Light|SetIntensity _rectlight 1e+02)
  (Utilities|FlowControl|Delay 0.5)
  (Rendering|Components|Light|SetIntensity _rectlight 1e+03))

(event EventBeginPlay)

(event Collision|EventActorBeginOverlap
  (params (OtherActor :type Actor%20Object%20Reference)))

(event EventTick
  (params (DeltaSeconds :type Float%20%28single-precision%29))
  (bind _rectlight (Variables|Default|GetRectLight))
  (bind _returnvalue (Transformation|GetWorldRotation _rectlight))
  (Transformation|SetRelativeRotation _rectlight (Math|Rotator|MakeRotator (.roll _returnvalue) (.pitch _returnvalue) (+ (.yaw _returnvalue) (* DeltaSeconds 1e+02))) false false)
  (if (Variables|Default|GetSpookIsNear)
    (CallFunction|Flicker)
    (Utilities|FlowControl|Delay (Math|Random|RandomFloatinRange 5.0 3e+01))))

(fn ConstructionScript)