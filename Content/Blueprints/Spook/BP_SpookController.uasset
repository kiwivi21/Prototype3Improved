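; AI controller for the Spook that runs BT_Spook and feeds its blackboard, starting with the player as target.
; Sight perception sets or clears Target; losing sight keeps PlayerLoc tracking the player's true position for a grace period before clearing it.
; Tick searches all BP_Vent actors every frame to write ClosestVent, and StartWander raises ShouldWander for WanderTime.
; LastSeenLoc is only written at BeginPlay, as its sight-update node is unconnected.
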(event OnTargetPerceptionUpdated(AIPerception)
  (params (Actor :type Actor%20Object%20Reference) (Stimulus :type AI%20Stimulus%20Structure))
  (bind _returnvalue (Class|AIPerceptionSystem|GetSenseClassforStimulus Stimulus))
  (if (== _returnvalue "/Script/AIModule.AISense_Sight")
    (CallFunction|HandleSight Actor Stimulus)))

(event Custom|StartWander
  (AI|Components|Blackboard|SetValueasBool (Variables|Default|GetBlackboard) (Utilities|Name|MakeLiteralName "ShouldWander") true)
  (Utilities|FlowControl|Delay (Variables|Default|GetWanderTime))
  (AI|Components|Blackboard|SetValueasBool (Variables|Default|GetBlackboard) (Utilities|Name|MakeLiteralName "ShouldWander") false)
  (Variables|Default|SetShouldWander false))

(event Custom|LostSightOfPlayer
  (Variables|Default|SetShouldKnowPlayerLoc true)
  (Utilities|FlowControl|Delay 15.0)
  (AI|Components|Blackboard|ClearValue (Variables|Default|GetBlackboard) (Utilities|Name|MakeLiteralName "PlayerLoc"))
  (Variables|Default|SetShouldKnowPlayerLoc false))

(event EventBeginPlay
  (bind _returnvalue (Game|GetPlayerCharacter 0))
  (AI|RunBehaviorTree "/Game/Blueprints/Spook/BT_Spook.BT_Spook")
  (AI|Components|Blackboard|SetValueasVector (Variables|Default|GetBlackboard) (Utilities|Name|MakeLiteralName "LastSeenLoc") (Transformation|GetWorldLocation (Variables|/Script/Engine.Actor|GetRootComponent _returnvalue)))
  (AI|Components|Blackboard|SetValueasObject (Variables|Default|GetBlackboard) (Utilities|Name|MakeLiteralName "Target") _returnvalue))

(event EventTick
  (params (DeltaSeconds :type Float%20%28single-precision%29))
  (bind _blackboard (Variables|Default|GetBlackboard))
  (bind _outactors (Actor|GetAllActorsOfClass "/Game/Blueprints/Spook/BP_Vent.BP_Vent_C"))
  (AI|Components|Blackboard|SetValueasObject _blackboard (Utilities|Name|MakeLiteralName "ClosestVent") (.ReturnValue (Actor|FindNearestActor (Transformation|GetActorLocation) _outactors)))
  (if (Variables|Default|GetShouldKnowPlayerLoc)
    (AI|Components|Blackboard|SetValueasVector _blackboard (Utilities|Name|MakeLiteralName "PlayerLoc") (Transformation|GetActorLocation (Game|GetPlayerCharacter 0)))))

(fn ConstructionScript)

(fn HandleSight
  (params (Actor :type Actor%20Object%20Reference) (Stimulus :type AI%20Stimulus%20Structure))
  (bind (_age _expirationage _strength _stimuluslocation _receiverlocation _tag _bsuccessfullysensed) (Utilities|Struct|BreakAIStimulus Stimulus))
  (if (== Actor (Game|GetPlayerCharacter 0))
    (AI|Components|Blackboard|SetValueasObject (Variables|Default|GetBlackboard) (Utilities|Name|MakeLiteralName "Target") (Utilities|SelectObject Actor 0 _bsuccessfullysensed))
    (if (not _bsuccessfullysensed)
      (CallFunction|LostSightOfPlayer))
    (else
      (return))))