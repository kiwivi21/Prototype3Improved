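; Behavior tree task for the Spook AI that, despite its name, moves the pawn toward the player character rather than a last-seen location.
; On either success or failure, it calls StartWander on every BP_SpookController in the level.
; The live path never calls FinishExecute; the LastSeenLoc move, blackboard clearing and ShouldWander logic sit in disconnected nodes.
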(event EventReceiveExecuteAI
  (params (OwnerController :type AI%20Controller%20Object%20Reference) (ControlledPawn :type Pawn%20Object%20Reference))
  (bind _blackboardcomponent (Class|AIController|UseBlackboard OwnerController "/Game/Blueprints/Spook/BB_Spook.BB_Spook"))
  (AI|AIMoveTo ControlledPawn "0, 0, 0" (Game|GetPlayerCharacter 0) 5.0 false
    (:OnSuccess
      (bind _outactors (Actor|GetAllActorsOfClass "/Game/Blueprints/Spook/BP_SpookController.BP_SpookController_C"))
      (for _array_element _outactors
        (Default|StartWander _array_element)))
    (:OnFail
      (bind _outactors_2 (Actor|GetAllActorsOfClass "/Game/Blueprints/Spook/BP_SpookController.BP_SpookController_C"))
      (for _array_element_2 _outactors_2
        (Default|StartWander _array_element_2)))))