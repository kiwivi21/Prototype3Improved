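; BP_Spook is a spook actor that casts Niagara tracer effects onto nearby surfaces and reacts to vents.
; On Tick, UpdateTracers runs a cooldown-limited line trace in a random direction between two radii; hits spawn an attached NS_SpookEnhanced fed start, offset impact point and normal.
; Overlapping a BP_Vent disables capsule collision and moves the capsule to a fixed height at its current XY.
; A blackboard ClosestVent clear exists but is unconnected.
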(event OnComponentBeginOverlap(CapsuleComponent)
  (params (OverlappedComponent :type Primitive%20Component%20Object%20Reference) (OtherActor :type Actor%20Object%20Reference) (OtherComp :type Primitive%20Component%20Object%20Reference) (OtherBodyIndex :type Integer) (bFromSweep :type Boolean) (SweepResult :type Hit%20Result%20Structure%20%28by%20ref%29))
  (bind _capsulecomponent (Variables|Collision|GetCapsuleComponent))
  (bind _returnvalue (Transformation|GetWorldLocation _capsulecomponent))
  (Utilities|Casting|CastToBP_Vent OtherActor)
  (Collision|SetCollisionEnabled (Variables|Collision|GetCapsuleComponent) "NoCollision")
  (Transformation|SetWorldLocation _capsulecomponent (Math|Vector|MakeVector (.x _returnvalue) (.y _returnvalue) 1e+03) true false))

(event EventBeginPlay)

(event Collision|EventActorBeginOverlap
  (params (OtherActor :type Actor%20Object%20Reference)))

(event EventTick
  (params (DeltaSeconds :type Float%20%28single-precision%29))
  (CallFunction|UpdateTracers))

(fn ConstructionScript)

(fn UpdateTracers
  (bind _returnvalue (Transformation|GetActorLocation))
  (if (>= (- (Utilities|Time|GetTimeSeconds) (Variables|Default|GetLastTrace)) (Variables|Default|GetTraceCoolDown))
    (Variables|Default|SetRandomDirection (Math|Random|RandomUnitVector))
    (bind _outhit (Collision|LineTraceByChannel (+ _returnvalue (* (Variables|Default|GetRandomDirection) (Variables|Default|GetMinRadius))) (+ _returnvalue (* (Variables|Default|GetRandomDirection) (Variables|Default|GetMaxRadius))) "TraceTypeQuery1" false 0 "None" true "(R=1.000000,G=0.000000,B=0.000000,A=1.000000)" "(R=0.000000,G=1.000000,B=0.000000,A=1.000000)" (Variables|Default|GetTraceCoolDown)))
    (Variables|Default|SetLastTrace (Utilities|Time|GetTimeSeconds))
    (if (.bBlockingHit (Collision|BreakHitResult _outhit))
      (bind _returnvalue_2 (Niagara|SpawnSystemAttached "/Game/Blueprints/Spook/NS_SpookEnhanced.NS_SpookEnhanced" (Variables|Default|GetSphere) "None" "0, 0, 0" "0, 0, 0" "KeepRelativeOffset" false))
      (Niagara|SetNiagaraVariable(Vector3) _returnvalue_2 "StartPos" (* (Variables|Default|GetRandomDirection) (Variables|Default|GetMinRadius)))
      (Niagara|SetNiagaraVariable(Vector3) _returnvalue_2 "EndPos" (+ (.ImpactPoint (Collision|BreakHitResult _outhit)) (* (.ImpactNormal (Collision|BreakHitResult _outhit)) (LocalVariables|GetImpactOffset))))
      (Niagara|SetNiagaraVariable(Vector3) _returnvalue_2 "ImpactNormal" (.ImpactNormal (Collision|BreakHitResult _outhit))))))