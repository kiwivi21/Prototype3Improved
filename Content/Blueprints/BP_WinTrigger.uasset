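; Level trigger actor that ends the horror game with a win once the quest number reaches 7 or higher.
; Tick polls the game instance's quest progress and activates the helicopter SFX at that threshold.
; When the first-person character then overlaps WinTrigger, it pauses the game, switches to UI input, swaps all widgets for WBP_Win and plays music.
; Chained title and button fades finish by revealing the buttons and mouse cursor.
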(event OnComponentBeginOverlap(WinTrigger)
  (params (OverlappedComponent :type Primitive%20Component%20Object%20Reference) (OtherActor :type Actor%20Object%20Reference) (OtherComp :type Primitive%20Component%20Object%20Reference) (OtherBodyIndex :type Integer) (bFromSweep :type Boolean) (SweepResult :type Hit%20Result%20Structure%20%28by%20ref%29))
  (bind _returnvalue (Game|GetPlayerController 0))
  (bind _asbp_horror_instance (Utilities|Casting|CastToBP_HorrorInstance (Game|GetGameInstance)))
  (if (>= (Variables|/Game/Blueprints/BP_HorrorInstance.BP_HorrorInstance_C|GetQuestNumber _asbp_horror_instance) 7)
    (Development|PrintString "true1")
    (if (== (Utilities|GetClass OtherActor) "/Game/FirstPerson/Blueprints/BP_FirstPersonCharacter.BP_FirstPersonCharacter_C")
      (Development|PrintString "true2")
      (Input|SetInputModeUIOnly _returnvalue 0 "DoNotLock" false)
      (Game|SetGamePaused true)
      (Viewport|RemoveAllWidgets)
      (bind _returnvalue_2 (UserInterface|CreateWidget "/Game/Blueprints/WBP_Win.WBP_Win_C"))
      (UserInterface|Viewport|AddtoViewport _returnvalue_2 0)
      (Audio|PlaySound2D "/Game/Assets/Sounds/MainMenu.MainMenu" 1.0 1.0 0.0 0 0)
      (Components|Animation|PlayAnimation _returnvalue_2 (Variables|/Game/Blueprints/WBP_Win.WBP_Win_C|GetTitleFade _returnvalue_2) 0.0
        (:Finished
          (Components|Animation|PlayAnimation _returnvalue_2 (Variables|/Game/Blueprints/WBP_Win.WBP_Win_C|GetButtonFade _returnvalue_2) 0.0
            (:Finished
              (Widget|SetVisibility (Variables|/Game/Blueprints/WBP_Win.WBP_Win_C|GetButtonArray _returnvalue_2) "Visible")
              (Variables|/Script/Engine.PlayerController|SetbShowMouseCursor _returnvalue true)))))
      (else
        (Development|PrintString "false2")))
    (else
      (Development|PrintString "false1"))))

(event EventBeginPlay)

(event Collision|EventActorBeginOverlap
  (params (OtherActor :type Actor%20Object%20Reference)))

(event EventTick
  (params (DeltaSeconds :type Float%20%28single-precision%29))
  (bind _questnum (Class|BPIInstanceControl|GetQuestNum(Message) (Game|GetGameInstance)))
  (if (and (!= (Components|Activation|IsActive (Variables|Default|GetSFX_Helicopter)) true) (>= _questnum 7))
    (Components|Activation|SetActive (Variables|Default|GetSFX_Helicopter) true false)))

(fn ConstructionScript)