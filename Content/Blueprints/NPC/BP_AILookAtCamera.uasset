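; Quest-giver NPC that advances the fuse and antenna quests when the player enters its TalkCollision.
; On overlap it checks QuestNumber in BP_HorrorInstance: quest 1 advances to 2 and quest 3 to 4.
; Each step prints a hint, updates the quest text, saves through the player character and plays Reuben's voice audio.
; The first conversation alternates Reuben's lines with replies played at world origin, timed by hard-coded delays.
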(event OnComponentBeginOverlap(TalkCollision)
  (params (OverlappedComponent :type Primitive%20Component%20Object%20Reference) (OtherActor :type Actor%20Object%20Reference) (OtherComp :type Primitive%20Component%20Object%20Reference) (OtherBodyIndex :type Integer) (bFromSweep :type Boolean) (SweepResult :type Hit%20Result%20Structure%20%28by%20ref%29))
  (bind _returnvalue (Game|GetPlayerCharacter 0))
  (if (== OtherActor _returnvalue)
    (bind _asbp_horror_instance (Utilities|Casting|CastToBP_HorrorInstance (Game|GetGameInstance)))
    (if (== (Variables|/Game/Blueprints/BP_HorrorInstance.BP_HorrorInstance_C|GetQuestNumber _asbp_horror_instance) 1)
      (Development|PrintString "We need to get the elevator working, find another working fuse! PLEASE!")
      (Variables|/Game/Blueprints/BP_HorrorInstance.BP_HorrorInstance_C|SetQuestString _asbp_horror_instance "Quest 2: Find a fuse to complete the fusebox")
      (Variables|/Game/Blueprints/BP_HorrorInstance.BP_HorrorInstance_C|SetQuestNumber _asbp_horror_instance 2)
      (bind _asbp_first_person_character (Utilities|Casting|CastToBP_FirstPersonCharacter _returnvalue))
      (Default|Save _asbp_first_person_character)
      (Audio|Components|Audio|Play (Variables|Default|GetReubenAudio1) 0.0)
      (Utilities|FlowControl|Delay 24.0)
      (Audio|PlaySoundatLocation "/Game/Assets/Sounds/Player/PlayerVoice/3_-_What_do_we_need.3_-_What_do_we_need" "0, 0, 0" "0, 0, 0" 1.0 1.0 0.0 0 0 0 0)
      (Utilities|FlowControl|Delay 5.0)
      (Audio|Components|Audio|Play (Variables|Default|GetReubenAudio2) 0.0)
      (Utilities|FlowControl|Delay 14.0)
      (Audio|PlaySoundatLocation "/Game/Assets/Sounds/Player/PlayerVoice/4_-_hang_tight.4_-_hang_tight" "0, 0, 0" "0, 0, 0" 1.0 1.0 0.0 0 0 0 0)
      (Utilities|FlowControl|Delay 3.5)
      (Audio|Components|Audio|Play (Variables|Default|GetReubenAudio3) 0.0)
      (elif (== (Variables|/Game/Blueprints/BP_HorrorInstance.BP_HorrorInstance_C|GetQuestNumber _asbp_horror_instance) 3)
        (Development|PrintString "The power is on, but the Antenna busted! There should be a spare on the second floor... let's hope there's enough power for the elevator to work")
        (Variables|/Game/Blueprints/BP_HorrorInstance.BP_HorrorInstance_C|SetQuestString _asbp_horror_instance "Quest 4: Find a Antenna on the 2nd floor")
        (Variables|/Game/Blueprints/BP_HorrorInstance.BP_HorrorInstance_C|SetQuestNumber _asbp_horror_instance 4)
        (bind _asbp_first_person_character_2 (Utilities|Casting|CastToBP_FirstPersonCharacter _returnvalue))
        (Default|Save _asbp_first_person_character_2)
        (Audio|Components|Audio|Play (Variables|Default|GetReubenAudio4) 0.0)))))

(event EventBeginPlay)

(event Collision|EventActorBeginOverlap
  (params (OtherActor :type Actor%20Object%20Reference)))

(event EventTick
  (params (DeltaSeconds :type Float%20%28single-precision%29)))

(fn ConstructionScript)