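; BP_DownElevator is an elevator Blueprint that caches open and closed positions for two sliding doors on BeginPlay.
; Its CloseDoors and Interact events are empty, so it currently does nothing further.
; Disconnected logic would play a sound once, call CloseDoors on BP_ElevatorDoors, then open Level1 after a delay.
; An unconnected Doors timeline holds the lerp that would slide both doors shut.
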(event Custom|CloseDoors)

(event EventBeginPlay
  (bind _doorright (Variables|Default|GetDoorRight))
  (bind _doorleft (Variables|Default|GetDoorLeft))
  (bind _relativelocation (Variables|/Script/Engine.SceneComponent|GetRelativeLocation _doorleft))
  (bind _relativelocation_2 (Variables|/Script/Engine.SceneComponent|GetRelativeLocation _doorright))
  (Variables|Default|SetDoorRightOpenPos (Variables|/Script/Engine.SceneComponent|GetRelativeLocation (Variables|Default|GetDoorRight)))
  (Variables|Default|SetDoorRightClosedPos (Math|Vector|MakeVector (+ (.x _relativelocation_2) -1.5e+02) (.y _relativelocation_2) (.z _relativelocation_2)))
  (Variables|Default|SetDoorLeftOpenPos (Variables|/Script/Engine.SceneComponent|GetRelativeLocation (Variables|Default|GetDoorLeft)))
  (Variables|Default|SetDoorLeftClosedPos (Math|Vector|MakeVector (+ (.x _relativelocation) 1.5e+02) (.y _relativelocation) (.z _relativelocation))))

(event EventInteract)

(fn ConstructionScript)