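; Elevator double doors that slide open and closed, opening automatically in a horror game once quest progress is past the start.
; BeginPlay treats the placed door positions as closed and derives open positions by offsetting each door sideways along its relative X.
; If the game instance's quest number is above zero, it opens them after a short delay.
; One Timeline lerps both doors, playing forward to close and in reverse to open.
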(event Custom|CloseDoors
  (bind _newtrack_0 (Timeline|Timeline PlayFromStart)
    (:Update
      (Transformation|SetRelativeLocation (Variables|Default|GetDoorRight) (Math|Vector|Lerp(Vector) (Variables|Default|GetRightOpenPos) (Variables|Default|GetRightClosedPos) _newtrack_0) false false)
      (Transformation|SetRelativeLocation (Variables|Default|GetDoorLeft) (Math|Vector|Lerp(Vector) (Variables|Default|GetLerftOpenPos) (Variables|Default|GetLeftClosedPos) _newtrack_0) false false))))

(event Custom|Open%20Doors
  (bind _newtrack_0 (Timeline|Timeline ReverseFromEnd)
    (:Update
      (Transformation|SetRelativeLocation (Variables|Default|GetDoorRight) (Math|Vector|Lerp(Vector) (Variables|Default|GetRightOpenPos) (Variables|Default|GetRightClosedPos) _newtrack_0) false false)
      (Transformation|SetRelativeLocation (Variables|Default|GetDoorLeft) (Math|Vector|Lerp(Vector) (Variables|Default|GetLerftOpenPos) (Variables|Default|GetLeftClosedPos) _newtrack_0) false false))))

(event EventBeginPlay
  (bind _doorleft (Variables|Default|GetDoorLeft))
  (bind _doorright (Variables|Default|GetDoorRight))
  (bind _relativelocation (Variables|/Script/Engine.SceneComponent|GetRelativeLocation _doorright))
  (bind _relativelocation_2 (Variables|/Script/Engine.SceneComponent|GetRelativeLocation _doorleft))
  (Variables|Default|SetRightOpenPos (Math|Vector|MakeVector (+ (.x _relativelocation) 1.1e+02) (.y _relativelocation) (.z _relativelocation)))
  (Variables|Default|SetRightClosedPos (Variables|/Script/Engine.SceneComponent|GetRelativeLocation (Variables|Default|GetDoorRight)))
  (Variables|Default|SetLerftOpenPos (Math|Vector|MakeVector (+ (.x _relativelocation_2) -1.1e+02) (.y _relativelocation_2) (.z _relativelocation_2)))
  (Variables|Default|SetLeftClosedPos (Variables|/Script/Engine.SceneComponent|GetRelativeLocation (Variables|Default|GetDoorLeft)))
  (bind _asbp_horror_instance (Utilities|Casting|CastToBP_HorrorInstance (Game|GetGameInstance)))
  (if (> (Variables|/Game/Blueprints/BP_HorrorInstance.BP_HorrorInstance_C|GetQuestNumber _asbp_horror_instance) 0)
    (Utilities|FlowControl|Delay 1.0)
    (CallFunction|OpenDoors)))

(fn ConstructionScript)