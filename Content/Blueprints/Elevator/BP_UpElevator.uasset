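; BP_UpElevator is a one-use interactable elevator that closes its doors and moves the player to Level2.
; BeginPlay caches each door's relative location as open and derives closed positions by offsetting X in opposite directions.
; Interact sets the Used guard, plays a 2D door sound and calls CloseDoors, which slides both doors with a Timeline-driven lerp.
; After a fixed delay, it opens Level2 by object reference.
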(event Custom|CloseDoors
  (bind _newtrack_0 (Timeline|Doors Play)
    (:Update
      (Transformation|SetRelativeLocation (Variables|Default|GetDoorRight) (Math|Vector|Lerp(Vector) (Variables|Default|GetDoorRightOpenPos) (Variables|Default|GetDoorRightClosedPos) _newtrack_0) false false)
      (Transformation|SetRelativeLocation (Variables|Default|GetDoorLeft) (Math|Vector|Lerp(Vector) (Variables|Default|GetDoorLeftOpenPos) (Variables|Default|GetDoorLeftClosedPos) _newtrack_0) false false))))

(event EventBeginPlay
  (bind _doorright (Variables|Default|GetDoorRight))
  (bind _doorleft (Variables|Default|GetDoorLeft))
  (bind _relativelocation (Variables|/Script/Engine.SceneComponent|GetRelativeLocation _doorleft))
  (bind _relativelocation_2 (Variables|/Script/Engine.SceneComponent|GetRelativeLocation _doorright))
  (Variables|Default|SetDoorRightOpenPos (Variables|/Script/Engine.SceneComponent|GetRelativeLocation (Variables|Default|GetDoorRight)))
  (Variables|Default|SetDoorRightClosedPos (Math|Vector|MakeVector (+ (.x _relativelocation_2) -1.5e+02) (.y _relativelocation_2) (.z _relativelocation_2)))
  (Variables|Default|SetDoorLeftOpenPos (Variables|/Script/Engine.SceneComponent|GetRelativeLocation (Variables|Default|GetDoorLeft)))
  (Variables|Default|SetDoorLeftClosedPos (Math|Vector|MakeVector (+ (.x _relativelocation) 1.5e+02) (.y _relativelocation) (.z _relativelocation))))

(event EventInteract
  (if (not (Variables|Default|GetUsed))
    (Variables|Default|SetUsed true)
    (Audio|PlaySound2D "/Game/Assets/Sounds/Ambience/155897__tiptoe84__elevatordoor2.155897__tiptoe84__elevatordoor2" 2.0 1.0 2.0 0 0)
    (CallFunction|CloseDoors)
    (Utilities|FlowControl|Delay 4.0)
    (Game|OpenLevel(byObjectReference) "/Game/Levels/Level2.Level2")))

(fn ConstructionScript)