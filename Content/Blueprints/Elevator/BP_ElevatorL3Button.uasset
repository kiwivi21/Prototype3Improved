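; Elevator button that takes the player to Level 3 when interacted with, provided they carry a keycard.
; It searches the HorrorInstance game instance's inventory names for "Keycard", then marks itself used and plays a door sound.
; It closes the BP_ElevatorDoors actor it finds and opens Level 3 after a short delay.
; The "No keycard?" debug print follows the search loop, even when a keycard is found.
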(event EventBeginPlay)

(event Collision|EventActorBeginOverlap
  (params (OtherActor :type Actor%20Object%20Reference)))

(event EventTick
  (params (DeltaSeconds :type Float%20%28single-precision%29)))

(event EventInteract
  (if (not (Variables|Default|GetUsed))
    (bind _asbp_horror_instance (Utilities|Casting|CastToBP_HorrorInstance (Game|GetGameInstance)))
    (for _array_element (Variables|/Game/Blueprints/BP_HorrorInstance.BP_HorrorInstance_C|GetNamesInInventory _asbp_horror_instance)
      (if (Utilities|Enum|Equal(Enum) _array_element "Keycard")
        (Variables|Default|SetUsed true)
        (Audio|PlaySound2D "/Game/Assets/Sounds/Ambience/155897__tiptoe84__elevatordoor2.155897__tiptoe84__elevatordoor2" 1.0 1.0 2.0 0 0)
        (bind _returnvalue (Actor|GetActorOfClass "/Game/Blueprints/Elevator/BP_ElevatorDoors.BP_ElevatorDoors_C"))
        (Utilities|IsValid _returnvalue
          (:Is%20Valid
            (Default|CloseDoors _returnvalue)
            (Utilities|FlowControl|Delay 4.0)
            (Game|OpenLevel(byObjectReference) "/Game/Levels/Level3.Level3")))))
    (Development|PrintString "No keycard?")))

(fn ConstructionScript)