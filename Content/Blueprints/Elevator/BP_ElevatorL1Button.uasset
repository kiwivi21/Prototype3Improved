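; BP_ElevatorL1Button is an interactable elevator button that sends the player to Level1A.
; Interact works once, guarded by a Used flag, and plays an elevator door sound.
; It finds the BP_ElevatorDoors actor in the level and, if valid, closes the doors and plays the WBP_Fade FadeIn animation in reverse.
; After a short delay, it opens the level.
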(event EventBeginPlay)

(event Collision|EventActorBeginOverlap
  (params (OtherActor :type Actor%20Object%20Reference)))

(event EventTick
  (params (DeltaSeconds :type Float%20%28single-precision%29)))

(event EventInteract
  (if (not (Variables|Default|GetUsed))
    (Variables|Default|SetUsed true)
    (Audio|PlaySound2D "/Game/Assets/Sounds/Ambience/155897__tiptoe84__elevatordoor2.155897__tiptoe84__elevatordoor2" 1.0 1.0 2.0 0 0)
    (bind _returnvalue (Actor|GetActorOfClass "/Game/Blueprints/Elevator/BP_ElevatorDoors.BP_ElevatorDoors_C"))
    (Utilities|IsValid _returnvalue
      (:Is%20Valid
        (Default|CloseDoors _returnvalue)
        (bind _returnvalue_2 (UserInterface|CreateWidget "/Game/Blueprints/WBP_Fade.WBP_Fade_C"))
        (UserInterface|Viewport|AddtoViewport _returnvalue_2 0)
        (UserInterface|Animation|PlayAnimation _returnvalue_2 (Variables|/Game/Blueprints/WBP_Fade.WBP_Fade_C|GetFadeIn _returnvalue_2) 0.0 1 "Reverse" 1.0 false)
        (Utilities|FlowControl|Delay 4.0)
        (Game|OpenLevel(byObjectReference) "/Game/Levels/Level1A.Level1A")))))

(fn ConstructionScript)