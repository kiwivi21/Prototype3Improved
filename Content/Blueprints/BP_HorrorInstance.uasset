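; BP_HorrorInstance holds shared state for a horror game: audio volume settings and the names of inventory items.
; The SendVolume event stores music, SFX and voice levels, and GetVolume returns all three.
; AddNameToList records an item's unique inventory name without duplicates.
; It only stores these values and does not apply the volumes to audio itself.
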(event EventSendVolume
  (params (Music :type Float%20%28double-precision%29) (SFX :type Float%20%28double-precision%29) (Voice :type Float%20%28double-precision%29))
  (Variables|Default|SetBGMVolume Music)
  (Variables|Default|SetSFXVolume SFX)
  (Variables|Default|SetVoiceVolume Voice))

(fn AddNametoList
  (params (Item :type BP%20Parent%20Pickup%20Object%20Reference))
  (Utilities|Array|AddUnique (Variables|Default|GetNamesInInventory) (Variables|/Game/Blueprints/Inventory/ItemsForInventory/BP_ParentPickup.BP_ParentPickup_C|GetUniqueNameForInventory Item))
  (return))

(fn GetVolume
  (return (Variables|Default|GetBGMVolume) (Variables|Default|GetSFXVolume) (Variables|Default|GetVoiceVolume)))